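; BP_PingPong is an animated ping-pong prop that plays a one-shot animation when triggered by the GM_Barrels game mode.
; On BeginPlay it binds to the game mode's PingPong event dispatcher, whose callback plays Pingpong_Anim on the Pingpong mesh without looping.
; Every Tick it reads a custom transform attribute from a bone of that mesh and applies it as the Paddle's world transform.
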(event `self.ReceiveBeginPlay`
  (bind _asgm_barrels (cast `/Game/Blueprints/GM_Barrels` (`GameplayStatics.GetGameMode`)))
  (set `self.GM_Barrels` _asgm_barrels)
  (add `/Game/Blueprints/GM_Barrels.ED_PingPong` (`self.GM_Barrels`) (delegate `CE_PlayAnimation`)))

(event `CE_PlayAnimation`
  (`SkeletalMeshComponent.PlayAnimation` (`self.pingpong`) "/Game/Animation/PingPong/pingpong_Anim.pingpong_Anim" false))

(event `self.ReceiveTick`
  (params (DeltaSeconds :type "Float (single-precision)"))
  (bind _outvalue (`SkeletalMeshComponent.GetTransformAttribute` :`self` (`self.pingpong`) :`BoneName` (`self.Bone Name`) :`AttributeName` (`self.Attribute Name`)))
  (`SceneComponent.K2_SetWorldTransform` (`self.Paddle`) _outvalue false false))

(fn `PlayAnimation`)

(fn `UserConstructionScript`)