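; Barrel actor that randomizes its look and destroys itself when the Barrels game mode signals an explosion.
; The construction script creates a dynamic material instance on the barrel mesh and randomly applies one of three BaseColor, Normal and ARM texture sets.
; On BeginPlay it binds its explode event to the GM_Barrels dispatcher, so the game mode's broadcast destroys every bound barrel.
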(event `self.ReceiveBeginPlay`
  (bind _asgm_barrels (cast `/Game/Blueprints/GM_Barrels` (`GameplayStatics.GetGameMode`)))
  (set `self.As GM Barrels` _asgm_barrels)
  (add `/Game/Blueprints/GM_Barrels.ED_Explode` (`self.As GM Barrels`) (delegate `CE_Explode`)))

(event `CE_Explode`
  (`self.K2_DestroyActor`))

(fn `UserConstructionScript`
  (bind _returnvalue (`PrimitiveComponent.CreateDynamicMaterialInstance` (`self.SM_Barrel`) 0 "/Game/Textures/MI_Barrel.MI_Barrel" "None"))
  (set `self.DynaMat` _returnvalue)
  (switch `int` (`KismetMathLibrary.RandomIntegerInRange` 1 3)
    (:`1`
      (`MaterialInstanceDynamic.SetTextureParameterValue` (`self.DynaMat`) "BaseColor" "/Game/Textures/Barrel_BC_01.Barrel_BC_01")
      (`MaterialInstanceDynamic.SetTextureParameterValue` (`self.DynaMat`) "Normal" "/Game/Textures/Barrel_N_01.Barrel_N_01")
      (`MaterialInstanceDynamic.SetTextureParameterValue` (`self.DynaMat`) "ARM" "/Game/Textures/Barrel_ARM_01.Barrel_ARM_01"))
    (:`2`
      (`MaterialInstanceDynamic.SetTextureParameterValue` (`self.DynaMat`) "BaseColor" "/Game/Textures/Barrel_BC_02.Barrel_BC_02")
      (`MaterialInstanceDynamic.SetTextureParameterValue` (`self.DynaMat`) "Normal" "/Game/Textures/Barrel_N_02.Barrel_N_02")
      (`MaterialInstanceDynamic.SetTextureParameterValue` (`self.DynaMat`) "ARM" "/Game/Textures/Barrel_ARM_02.Barrel_ARM_02"))
    (:`3`
      (`MaterialInstanceDynamic.SetTextureParameterValue` (`self.DynaMat`) "BaseColor" "/Game/Textures/Barrel_BC_03.Barrel_BC_03")
      (`MaterialInstanceDynamic.SetTextureParameterValue` (`self.DynaMat`) "Normal" "/Game/Textures/Barrel_N_03.Barrel_N_03")
      (`MaterialInstanceDynamic.SetTextureParameterValue` (`self.DynaMat`) "ARM" "/Game/Textures/Barrel_ARM_03.Barrel_ARM_03"))))